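; Enemy character Blueprint with a floating health bar and a cone marker toggled by lock and unlock events.
; BeginPlay spawns a separate AiHealthBar actor above the enemy and sets the enemy as its widget's ParentEnemy.
; Tick moves the bar to follow above the enemy while preserving the bar's own rotation.
; The cone starts hidden in the construction script, shows on LockEvent and hides on UnlockEvent.
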(event `self.LockEvent`
  (`SceneComponent.SetVisibility` (`self.Cone`) true false))

(event `self.UnlockEvent`
  (`SceneComponent.SetVisibility` (`self.Cone`) false false))

(event `self.ReceiveBeginPlay`
  (bind _returnvalue (`self.GetTransform`))
  (bind _returnvalue_2 (`|SpawnActorFromClass` "/Game/BluePrints/Enemy/AIHealthBar.AiHealthBar_C" (`KismetMathLibrary.MakeTransform` (`KismetMathLibrary.MakeVector` (.x (.location _returnvalue)) (.y (.location _returnvalue)) (+ (.z (.location _returnvalue)) 50.0)) (.rotation _returnvalue)) "Undefined" "OverrideRootScale" null null))
  (set `self.HealthBar` _returnvalue_2)
  (bind _asaihealth_bar_widget (cast `/Game/BluePrints/Enemy/AIHealthBarWidget` (`WidgetComponent.GetUserWidgetObject` (`/Game/BluePrints/Enemy/AIHealthBar.AiHealthBarWidget` _returnvalue_2))))
  (set `/Game/BluePrints/Enemy/AIHealthBarWidget.Parent Enemy` self _asaihealth_bar_widget))

(event `self.ReceiveTick`
  (params (DeltaSeconds :type "Float (single-precision)"))
  (bind _returnvalue (`self.GetTransform`))
  (`self.K2_SetActorTransform` (`self.HealthBar`) (`KismetMathLibrary.MakeTransform` (`KismetMathLibrary.MakeVector` (.x (.location _returnvalue)) (.y (.location _returnvalue)) (+ (.z (.location _returnvalue)) 50.0)) (`self.K2_GetActorRotation` (`self.HealthBar`))) false false))

(fn `UserConstructionScript`
  (`SceneComponent.SetVisibility` (`self.Cone`) false false))