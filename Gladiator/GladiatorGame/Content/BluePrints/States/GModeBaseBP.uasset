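; Base game mode Blueprint that spawns enemies and handles the player's win and loss.
; SpawnEnemies creates an EnemyCharacBP with EnemyBehaviourTree at every EnemySpawnPoint.
; PlayerWin and PlayerLose show their end widget, disable input (on the character for a win, the controller for a loss), show the cursor and stop all EnemyAIBP movement and brain logic.
; Their repeat guards are set inside the AI loop, so remain unset without AI controllers.
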(event `self.SpawnEnemies`
  (bind _outactors (`GameplayStatics.GetAllActorsOfClass` "/Game/BluePrints/Spawner/EnemySpawnPoint.EnemySpawnPoint_C"))
  (for _array_element _outactors
    (`AIBlueprintHelperLibrary.SpawnAIFromClass` "/Game/BluePrints/Enemy/EnemyCharacBP.EnemyCharacBP_C" "/Game/BluePrints/Enemy/EnemyBehaviourTree.EnemyBehaviourTree" (`SceneComponent.K2_GetComponentLocation` (`/Game/BluePrints/Spawner/EnemySpawnPoint.SpawnPoint` _array_element)))))

(event `self.ReceiveBeginPlay`)

(event `self.PlayerWin`
  (bind _returnvalue (`GameplayStatics.GetPlayerController` 0))
  (if (not (`self.IsGameWinSet`))
    (bind _returnvalue_2 (`|CreateWidget` "/Game/BluePrints/HUD/GameWin.GameWin_C"))
    (`UserWidget.AddToViewport` _returnvalue_2 0)
    (`Widget.SetVisibility` _returnvalue_2 "Visible")
    (`self.DisableInput` (`GameplayStatics.GetPlayerCharacter` 0) _returnvalue)
    (set `PlayerController.bShowMouseCursor` true _returnvalue)
    (bind _outactors (`GameplayStatics.GetAllActorsOfClass` "/Game/BluePrints/Enemy/EnemyAIBP.EnemyAIBP_C"))
    (for _array_element _outactors
      (`Controller.StopMovement` _array_element)
      (`BrainComponent.StopLogic` (`AIController.BrainComponent` _array_element) "GameOver")
      (set `self.IsGameWinSet` true))))

(event `self.PlayerLose`
  (bind _returnvalue (`GameplayStatics.GetPlayerController` 0))
  (if (not (`self.IsGameOverSet`))
    (bind _returnvalue_2 (`|CreateWidget` "/Game/BluePrints/HUD/GameOver.GameOver_C"))
    (`UserWidget.AddToViewport` _returnvalue_2 0)
    (`Widget.SetVisibility` _returnvalue_2 "Visible")
    (`self.DisableInput` _returnvalue _returnvalue)
    (set `PlayerController.bShowMouseCursor` true _returnvalue)
    (bind _outactors (`GameplayStatics.GetAllActorsOfClass` "/Game/BluePrints/Enemy/EnemyAIBP.EnemyAIBP_C"))
    (for _array_element _outactors
      (`Controller.StopMovement` _array_element)
      (`BrainComponent.StopLogic` (`AIController.BrainComponent` _array_element) "GameOver")
      (set `self.IsGameOverSet` true))))

(fn `UserConstructionScript`)