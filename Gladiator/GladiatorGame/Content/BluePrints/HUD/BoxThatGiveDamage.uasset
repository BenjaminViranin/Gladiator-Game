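; BoxThatGiveDamage is an actor that deals fixed damage to characters that hit it.
; Its Hit event casts the other actor to GCharacter, then EnemyCharacBP, and calls HandleTakeAnyDamage directly on that character's HealthComponent, ignoring anything else.
; An apparently unfinished CreateHitWidget function, uncalled here, only records a start time when no hit screen exists yet.
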(event `self.ReceiveHit`
  (params (MyComp :type "PrimitiveComponent Object Reference") (Other :type "Actor Object Reference") (OtherComp :type "PrimitiveComponent Object Reference") (bSelfMoved :type Boolean) (HitLocation :type "Vector Structure") (HitNormal :type "Vector Structure") (NormalImpulse :type "Vector Structure") (Hit :type "HitResult Structure (by ref)"))
  (bind _asgcharacter (cast `GCharacter` Other)
    (:`then`
      (`GHealthComponent.HandleTakeAnyDamage` (`GCharacter.HealthComponent` _asgcharacter) _asgcharacter 10.0 null null null))
    (:`CastFailed`
      (bind _asenemy_charac_bp (cast `/Game/BluePrints/Enemy/EnemyCharacBP` Other))
      (`GHealthComponent.HandleTakeAnyDamage` (`GEnemyCharacter.HealthComponent` _asenemy_charac_bp) _asenemy_charac_bp 10.0 null null null))))

(fn `CreateHitWidget`
  (if (not (`self.HitScreenAlreadyCreated`))
    (set `self.TimeAtStart` (`GameplayStatics.GetTimeSeconds`))))

(fn `UserConstructionScript`)